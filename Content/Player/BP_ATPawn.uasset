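; BP_ATPawn is the player pawn Blueprint, which applies saved player settings for gun visibility and camera field of view.
; On BeginPlay, LoadSettings reads the BP_SettingsSave held by BP_ATGameInstance and stops if either cast fails.
; It passes the saved values to ShowHideGun, which toggles the current weapon's mesh and its children, and to SetFOV, which adjusts the FPPCamera.
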(event `self.ReceiveBeginPlay`
  (`self.LoadSettings`))

(fn `LoadSettings`
  (bind _asbp_atgame_instance (cast `/Game/BP_ATGameInstance` (`GameplayStatics.GetGameInstance`)))
  (bind _asbp_settings_save (cast `/Game/BP_SettingsSave` (`/Game/BP_ATGameInstance.SaveRef` _asbp_atgame_instance)))
  (`self.ShowHideGun` (`/Game/BP_SettingsSave.ShowGun` _asbp_settings_save))
  (`self.SetFOV` (`/Game/BP_SettingsSave.FOV` _asbp_settings_save)))

(fn `SetFOV`
  (params (FOV :type "Float (double-precision)"))
  (`CameraComponent.SetFieldOfView` (`self.FPPCamera`) FOV))

(fn `ShowHideGun`
  (params (Visible :type Boolean))
  (`SceneComponent.SetVisibility` (`ATBaseWeapon.WeaponMesh` (`ATWeaponComponent.GetCurrentWeapon` (`self.WeaponComponent`))) Visible true))

(fn `UserConstructionScript`)