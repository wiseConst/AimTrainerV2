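; BP_ConeEnemy is an enemy that slides its static mesh back and forth along world Y, starting in a random direction.
; Tick applies a fixed per-frame offset, not scaled by delta time, while a retrigger-ignoring Delay flips Direction about every two seconds.
; When actor Y leaves its bounds, the ChangedDirection flag governs whether to reverse immediately or keep moving and flip after the delay.
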(event `self.ReceiveBeginPlay`
  (if (`KismetMathLibrary.RandomBool`)
    (set `self.Direction` 1.0)
    (else
      (set `self.Direction` -1.0))))

(event `self.ReceiveTick`
  (params (DeltaSeconds :type "Float (single-precision)"))
  (bind (_returnvalue_x _returnvalue_y) (`KismetMathLibrary.BreakVector` (`self.K2_GetActorLocation`)))
  (if (`KismetMathLibrary.InRange_FloatFloat` _returnvalue_y -1600.0 1600.0)
    (`SceneComponent.K2_AddWorldOffset` (`self.StaticMeshComponent`) (`KismetMathLibrary.MakeVector` 0.0 (* (`self.Direction`) 10.0)) false false)
    (`KismetSystemLibrary.Delay` 2.0)
    (set `self.Direction` (* (`self.Direction`) -1.0))
    (set `self.ChangedDirection` true)
    (elif (`self.ChangedDirection`)
      (set `self.ChangedDirection` false)
      (`SceneComponent.K2_AddWorldOffset` (`self.StaticMeshComponent`) (`KismetMathLibrary.MakeVector` 0.0 (* (`self.Direction`) 10.0)) false false)
      (`KismetSystemLibrary.Delay` 2.0)
      (set `self.Direction` (* (`self.Direction`) -1.0))
      (else
        (set `self.Direction` (* (`self.Direction`) -1.0))
        (set `self.ChangedDirection` true)
        (`SceneComponent.K2_AddWorldOffset` (`self.StaticMeshComponent`) (`KismetMathLibrary.MakeVector` 0.0 (* (`self.Direction`) 10.0)) false false)))))

(fn `UserConstructionScript`)