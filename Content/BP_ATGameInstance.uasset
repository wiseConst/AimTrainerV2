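; Game instance that restores the player's saved settings when the game initializes.
; On Init it loads the BP_SettingsSave slot, or creates one seeded from GameSettingsData defaults for gun visibility, FOV, sensitivity and volume.
; Either path applies the volume through a master sound mix class override and writes the save back to the slot.
; It then loads the engine's GameUserSettings; other saved values are not applied here.
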(event `self.ReceiveInit`
  (bind (_gamesettingsdata_sensitivitymultiplier _gamesettingsdata_soundvolume _gamesettingsdata_fov _gamesettingsdata_tilefrenzyenemycolor _gamesettingsdata_trackingenemycolor _gamesettingsdata_bshowgun) (break `GameSettingsData` (`self.GameSettingsData`)))
  (`|ExecutionSequence`
    (:`then_0`
      (bind _returnvalue (`GameplayStatics.DoesSaveGameExist` (`self.SaveSlot`)))
      (if _returnvalue
        (bind _returnvalue_2 (`GameplayStatics.LoadGameFromSlot` (`self.SaveSlot`)))
        (bind _output_get (set `self.SaveRef` _returnvalue_2))
        (bind _asbp_settings_save (cast `/Game/BP_SettingsSave` _output_get))
        (`GameplayStatics.SetSoundMixClassOverride` "/Game/Sounds/SoundMix_Master.SoundMix_Master" "/Game/Sounds/SC_Master.SC_Master" (`/Game/BP_SettingsSave.SoundVolume` _asbp_settings_save))
        (`GameplayStatics.PushSoundMixModifier` "/Game/Sounds/SoundMix_Master.SoundMix_Master")
        (`GameplayStatics.SaveGameToSlot` _asbp_settings_save (`self.SaveSlot`))
        (else
          (bind _returnvalue_3 (`GameplayStatics.CreateSaveGameObject` "/Game/BP_SettingsSave.BP_SettingsSave_C"))
          (bind _output_get_2 (set `self.SaveRef` _returnvalue_3))
          (bind _asbp_settings_save_2 (cast `/Game/BP_SettingsSave` _output_get_2))
          (set `/Game/BP_SettingsSave.ShowGun` _gamesettingsdata_bshowgun _asbp_settings_save_2)
          (set `/Game/BP_SettingsSave.FOV` _gamesettingsdata_fov _asbp_settings_save_2)
          (set `/Game/BP_SettingsSave.Sensitivity` _gamesettingsdata_sensitivitymultiplier _asbp_settings_save_2)
          (bind _output_get_3 (set `/Game/BP_SettingsSave.SoundVolume` _gamesettingsdata_soundvolume _asbp_settings_save_2))
          (`GameplayStatics.SetSoundMixClassOverride` "/Game/Sounds/SoundMix_Master.SoundMix_Master" "/Game/Sounds/SC_Master.SC_Master" _output_get_3)
          (`GameplayStatics.PushSoundMixModifier` "/Game/Sounds/SoundMix_Master.SoundMix_Master")
          (`GameplayStatics.SaveGameToSlot` _asbp_settings_save_2 (`self.SaveSlot`)))))
    (:`then_1`
      (bind _returnvalue_4 (`GameUserSettings.GetGameUserSettings`))
      (`GameUserSettings.LoadSettings` _returnvalue_4 false))))